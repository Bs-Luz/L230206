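; Player character Blueprint that handles basic movement, looking and jumping through Enhanced Input.
; On possession by a BP_PC controller, it adds the IMC_Input mapping context to that player's input subsystem.
; Move input is relative to control yaw only, with X driving forward and Y driving right.
; Look input feeds controller yaw and pitch, and jump starts on Triggered and stops on Completed.
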(event `self.ReceivePossessed`
  (params (NewController :type "Controller Object Reference"))
  (bind _asbp_pc (cast `/Game/Blueprints/BP_PC` NewController))
  (`EnhancedInputSubsystemInterface.AddMappingContext` (pcsubsystem `EnhancedInputLocalPlayerSubsystem` _asbp_pc) "/Game/Blueprints/Input/IMC_Input.IMC_Input" 0 (struct)))

(event `EnhancedInput|/Game/Blueprints/Input/IA_Move`
  (params (ActionValue :type "Vector2D Structure") (ElapsedSeconds :type "Float (double-precision)") (TriggeredSeconds :type "Float (double-precision)") (InputAction :type "InputAction Object Reference" :default "/Game/Blueprints/Input/IA_Move.IA_Move"))
  (bind (_returnvalue_roll _returnvalue_pitch _returnvalue_yaw) (`KismetMathLibrary.BreakRotator` (`self.GetControlRotation`)))
  (bind (_returnvalue_roll_2 _returnvalue_pitch_2 _returnvalue_yaw_2) (`KismetMathLibrary.BreakRotator` (`self.GetControlRotation`)))
  (:`Triggered`
    (`self.AddMovementInput` (`KismetMathLibrary.GetForwardVector` (`KismetMathLibrary.MakeRotator` 0.0 0.0 _returnvalue_yaw_2)) ActionValue_X)
    (`self.AddMovementInput` (`KismetMathLibrary.GetRightVector` (`KismetMathLibrary.MakeRotator` 0.0 0.0 _returnvalue_yaw)) ActionValue_Y)))

(event `EnhancedInput|/Game/Blueprints/Input/IA_Look`
  (params (ActionValue :type "Vector2D Structure") (ElapsedSeconds :type "Float (double-precision)") (TriggeredSeconds :type "Float (double-precision)") (InputAction :type "InputAction Object Reference" :default "/Game/Blueprints/Input/IA_Look.IA_Look"))
  (:`Triggered`
    (`self.AddControllerYawInput` ActionValue_X)
    (`self.AddControllerPitchInput` ActionValue_Y)))

(event `EnhancedInput|/Game/Blueprints/Input/IA_Jump`
  (params (ActionValue :type Boolean) (ElapsedSeconds :type "Float (double-precision)") (TriggeredSeconds :type "Float (double-precision)") (InputAction :type "InputAction Object Reference" :default "/Game/Blueprints/Input/IA_Jump.IA_Jump"))
  (:`Triggered`
    (`self.Jump`))
  (:`Completed`
    (`self.StopJumping`)))

(fn `UserConstructionScript`)